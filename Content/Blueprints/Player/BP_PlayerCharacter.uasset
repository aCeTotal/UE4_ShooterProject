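; Player character Blueprint that starts with a KA47 weapon and plays hit reactions.
; On BeginPlay, the authority adds the weapon to the PlayerInventory component.
; Point damage feeds PlayHitFX, which plays a random montage from HitReactionAnimations.
; The construction script adds the character to its SceneCaptureComponent2D show-only list, so the capture can render it in isolation.
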(event `self.ReceiveBeginPlay`
  (`/Engine/EditorBlueprintResources/ActorMacros.Switch Has Authority`
    (:`Authority`
      (`InventoryComponent.TryAddItemFromClass` (`self.PlayerInventory`) "/Game/Blueprints/Items/Weapons/BP_Weapon_KA47.BP_Weapon_KA47_C" 1))))

(event `self.ReceivePointDamage`
  (params (Damage :type "Float (single-precision)") (DamageType :type "DamageType Object Reference") (HitLocation :type "Vector Structure") (HitNormal :type "Vector Structure") (HitComponent :type "PrimitiveComponent Object Reference") (BoneName :type Name) (ShotFromDirection :type "Vector Structure") (InstigatedBy :type "Controller Object Reference") (DamageCauser :type "Actor Object Reference") (HitInfo :type "HitResult Structure (by ref)"))
  (`self.Play Hit FX` Damage DamageType true HitInfo))

(event `Play Hit FX`
  (params (Damage :type "Float (double-precision)") (DamageType :type "DamageType Object Reference") (`Point Damage?` :type Boolean) (Hit :type "HitResult Structure"))
  (bind _hitreactionanimations (`self.HitReactionAnimations`))
  (`self.PlayAnimMontage` (`|GetArrayItem` _hitreactionanimations (`KismetMathLibrary.RandomIntegerInRange` 0 (- (`KismetArrayLibrary.Array_Length` _hitreactionanimations) 1)))))

(fn `UserConstructionScript`
  (`KismetArrayLibrary.Array_AddUnique` (`SceneCaptureComponent.ShowOnlyActors` (`self.SceneCaptureComponent2D`)) self))